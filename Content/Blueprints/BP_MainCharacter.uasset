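; BP_MainCharacter is a character Blueprint that equips a weapon and plays melee attack and dodge animations.
; On BeginPlay, as test setup, it spawns BP_Weapon and snaps it to the mesh's SwordSocket.
; An attack event selects one of three montages from the Combo value, which this graph only reads.
; PlayJumpAnimMontage plays the dodge montage, despite its name.
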(event EventBeginPlay
  ;[1 1 1] Just for testing
  (bind _returnvalue (Game|SpawnActorfromClass "/Game/Blueprints/BP_Weapon.BP_Weapon_C" (Math|Conversions|ToTransform(Vector) (Transformation|GetSocketLocation (Variables|Character|GetMesh) "SwordSocket")) "Undefined" 0 0))
  (Transformation|AttachComponentToComponent _returnvalue (Variables|Character|GetMesh) "SwordSocket" "SnapToTarget" "SnapToTarget" "SnapToTarget" true))

(event EventPlayJumpAnimMontage
  (Animation|PlayAnimMontage "/Game/MyAssets/Animations/Paladin/AnimMontage_Dodge.AnimMontage_Dodge" 1.0 "None"))

(event EventPlayComboAnimMontage
  ;[1 1 1] Attacking System
  (switch int (Math|Conversions|ToInteger(Byte) (Variables|Default|GetCombo self))
    (:1
      (Animation|PlayAnimMontage "/Game/MyAssets/Animations/Paladin/AnimMontage_Attack1.AnimMontage_Attack1" 1.0 "None"))
    (:2
      (Animation|PlayAnimMontage "/Game/MyAssets/Animations/Paladin/AnimMontage_Attack2.AnimMontage_Attack2" 1.0 "None"))
    (:3
      (Animation|PlayAnimMontage "/Game/MyAssets/Animations/Paladin/AnimMontage_Attack3.AnimMontage_Attack3" 1.0 "None"))))

(fn ConstructionScript)